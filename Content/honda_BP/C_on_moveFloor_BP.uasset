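; Moving floor actor that shuttles its StaticMesh back and forth between StartPos and EndPos.
; On BeginPlay, the Control timeline plays at a rate of 1/MainRate, lerping the mesh's relative location without sweep.
; Each time it finishes, it waits three seconds and reverses direction, looping indefinitely.
; A leftover branch that heavily damages the player with an explosion sound is disconnected and never runs.
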(event `self.ReceiveBeginPlay`
  (`TimelineComponent.SetPlayRate` (`self.Control`) (/ 1.0 (`self.MainRate`)))
  (bind (_direction _rate) (`Timeline|Control` :!label _label)
    (:`Update`
      (`SceneComponent.K2_SetRelativeLocation` (`self.StaticMesh`) (`KismetMathLibrary.VLerp` (`self.StartPos`) (`self.EndPos`) _rate) false false))
    (:`Finished`
      (`KismetSystemLibrary.Delay` 3.0)
      (switch `ETimelineDirection` _direction
        (:`Forward`
          (goto _label :!via `Reverse`))
        (:`Backward`
          (goto _label))))))

(fn `UserConstructionScript`)